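; BP_ButtonInteraction is a button actor that changes color when something is near it and counts hits as a score.
; Overlap with the Trigger component swaps the Button's material to green, and ending the overlap turns it red.
; Each hit on the Button waits briefly, increments Score and prints it to the screen.
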(event OnComponentHit(Button)
  (params (HitComponent :type Primitive%20Component%20Object%20Reference) (OtherActor :type Actor%20Object%20Reference) (OtherComp :type Primitive%20Component%20Object%20Reference) (NormalImpulse :type Vector :default "0, 0, 0") (Hit :type Hit%20Result%20Structure%20%28by%20ref%29))
  (Utilities|FlowControl|Delay 0.05)
  (bind _output_get (Variables|Default|SetScore (+ (Variables|Default|GetScore) 1)))
  (Development|PrintString (Utilities|String|BuildString(Integer) "" "Score: " _output_get) true true "(R=0.000000,G=0.660000,B=1.000000,A=1.000000)" 5.0))

(event OnComponentBeginOverlap(Trigger)
  (params (OverlappedComponent :type Primitive%20Component%20Object%20Reference) (OtherActor :type Actor%20Object%20Reference) (OtherComp :type Primitive%20Component%20Object%20Reference) (OtherBodyIndex :type Integer) (bFromSweep :type Boolean) (SweepResult :type Hit%20Result%20Structure%20%28by%20ref%29))
  (Rendering|Material|SetMaterial (Variables|Default|GetButton) 0 "/Game/Task2/M_Green.M_Green"))

(event OnComponentEndOverlap(Trigger)
  (params (OverlappedComponent :type Primitive%20Component%20Object%20Reference) (OtherActor :type Actor%20Object%20Reference) (OtherComp :type Primitive%20Component%20Object%20Reference) (OtherBodyIndex :type Integer))
  (Rendering|Material|SetMaterial (Variables|Default|GetButton) 0 "/Game/Task2/M_Red.M_Red"))

(event EventBeginPlay)

(event Collision|EventActorBeginOverlap
  (params (OtherActor :type Actor%20Object%20Reference)))

(event EventTick
  (params (DeltaSeconds :type Float%20%28single-precision%29)))

(fn ConstructionScript)